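; BP_3rdCube is a trigger-driven cube that moves and reveals two texts when the first-person character overlaps its Collider.
; After a short delay, a timeline drives the Cube's relative Z location by a negatively scaled track value.
; Chained delays on the timeline's Update output make TextQQ visible, then TextAA.
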(event OnComponentBeginOverlap(Collider)
  (params (OverlappedComponent :type Primitive%20Component%20Object%20Reference) (OtherActor :type Actor%20Object%20Reference) (OtherComp :type Primitive%20Component%20Object%20Reference) (OtherBodyIndex :type Integer) (bFromSweep :type Boolean) (SweepResult :type Hit%20Result%20Structure%20%28by%20ref%29))
  (Utilities|Casting|CastToBP_FirstPersonCharacter OtherActor)
  (Utilities|FlowControl|Delay 1.0)
  (bind _newtrack_0 (Timeline|Timeline Play)
    (:Update
      (Transformation|SetRelativeLocation (Variables|Default|GetCube) (Math|Vector|MakeVector 0.0 0.0 (* _newtrack_0 -5.0)) false false)
      (Utilities|FlowControl|Delay 0.5)
      (Rendering|SetVisibility (Variables|Default|GetTextQQ) true false)
      (Utilities|FlowControl|Delay 0.8)
      (Rendering|SetVisibility (Variables|Default|GetTextAA) true false))))

(event EventBeginPlay)

(event Collision|EventActorBeginOverlap
  (params (OtherActor :type Actor%20Object%20Reference)))

(event EventTick
  (params (DeltaSeconds :type Float%20%28single-precision%29)))

(fn ConstructionScript)