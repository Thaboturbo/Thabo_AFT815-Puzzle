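; BP_Floor is a falling floor actor that drops away when the first-person character steps into its trigger box.
; The box overlap reveals a text render, waits briefly, then plays the BLock_Fall timeline.
; Timeline updates set the floor block's relative Z from the scaled FallDown track and start a one-second delay, after which the actor destroys itself.
; A debug string prints on any overlap, before the character cast.
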(event OnComponentBeginOverlap(Box)
  (params (OverlappedComponent :type Primitive%20Component%20Object%20Reference) (OtherActor :type Actor%20Object%20Reference) (OtherComp :type Primitive%20Component%20Object%20Reference) (OtherBodyIndex :type Integer) (bFromSweep :type Boolean) (SweepResult :type Hit%20Result%20Structure%20%28by%20ref%29))
  (Development|PrintString "Box been hit")
  (Utilities|Casting|CastToBP_FirstPersonCharacter OtherActor)
  (Rendering|SetVisibility (Variables|Default|GetTextRender) true false)
  (Utilities|FlowControl|Delay 0.5)
  (bind _fall_down (Timeline|BLock_Fall Play)
    (:Update
      (Transformation|SetRelativeLocation (Variables|Default|GetFloorBlock) (Math|Vector|MakeVector 0.0 0.0 (* _fall_down 1e+04)) false false)
      (Utilities|FlowControl|Delay 1.0)
      (Actor|DestroyActor))))

(fn ConstructionScript)